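; Game mode Blueprint for a Minecraft-style game that sets up the terrain noise and spawns the starting chunks.
; BeginPlay creates a Perlin FastNoise wrapper stored in Noise, then spawns a fixed 5x5 grid of Chunk actors around the origin, passing each its grid coordinates.
; GetPlayerChunk floors the player's location divided by 16, though chunks are spaced 1600 units apart.
; RestartLoading is an empty stub, and GetPlayerChunk is not called here.
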(event EventBeginPlay
  (Utilities|FlowControl|Sequence
    (:then_0
      (bind _returnvalue (Game|ConstructObjectfromClass "/Script/FastNoiseGenerator.FastNoiseWrapper"))
      (bind _output_get (Variables|Default|SetNoise _returnvalue))
      (Class|FastNoiseWrapper|SetupFastNoise _output_get "Perlin" 1337 0.05 "Quintic" "FBM" 3 2.0 0.5 0.45 "Euclidean" "CellValue"))
    (:then_1
      (for _index (range -2 2)
        (for _index_2 (range -2 2)
          (Game|SpawnActorfromClass "/Game/Minecraft/BluePrints/Chunk.Chunk_C" (Math|Transform|MakeTransform (* (Math|Vector|MakeVector (Math|Conversions|ToFloat(Integer) _index) (Math|Conversions|ToFloat(Integer) _index_2) 0.0) 1.6e+03) "0, 0, 0" "1.000000,1.000000,1.000000") "Undefined" "MultiplyWithRoot" 0 (Math|Vector|MakeVector (Math|Conversions|ToFloat(Integer) _index) (Math|Conversions|ToFloat(Integer) _index_2) 0.0) 0))))))

(fn ConstructionScript)

(fn RestartLoading)

(fn GetPlayerChunk
  (bind _returnvalue (Game|GetPlayerCharacter 0))
  (bind _returnvalue_2 (Transformation|GetActorLocation _returnvalue))
  (bind _returnvalue_3 (/ _returnvalue_2 16.0))
  (bind (_x _y) (Math|Vector|BreakVector _returnvalue_3))
  (Utilities|IsValid _returnvalue
    (:Is%20Valid
      (return (Math|Vector2D|MakeVector2D (Math|Conversions|ToFloat(Integer) (Math|Float|Floor _x)) (Math|Conversions|ToFloat(Integer) (Math|Float|Floor _y)))))
    (:Is%20Not%20Valid
      (return ""))))