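; Chunk actor for Minecraft-style terrain that builds one 16x16 surface layer of grass blocks on BeginPlay.
; Each block's height comes from the terrain game mode's 2D noise, sampled at chunk-offset coordinates and snapped to the block grid.
; MakeStaticMesh caches one instanced static mesh component per block data asset in a map, so blocks are added as instances.
; ShowChunk and HideChunk toggle actor visibility and track it in IsVisible.
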(event Custom|ShowChunk
  (Rendering|SetActorHiddenInGame false)
  (Variables|Default|SetIsVisible true))

(event Custom|HideChunk
  (Rendering|SetActorHiddenInGame true)
  (Variables|Default|SetIsVisible false))

(event EventBeginPlay
  (Utilities|FlowControl|Sequence
    (:then_0
      (bind _asgame_mode_terrain (Utilities|Casting|CastToGameModeTerrain (Game|GetGameMode)))
      (Variables|Default|SetAs%20Game%20Mode%20Terrain _asgame_mode_terrain))
    (:then_1
      (for _index (range 0 15)
        (for _index_2 (range 0 15)
          (bind _outputpin (CallFunction|MakeStaticMesh "/Game/Minecraft/DataAsset/GrassBlock.GrassBlock"))
          (Components|InstancedStaticMesh|AddInstance _outputpin (Math|Transform|MakeTransform (+ (* (Math|Vector|MakeVector (Math|Conversions|ToFloat(Integer) _index) (Math|Conversions|ToFloat(Integer) _index_2) 0.0) 1e+02) (Math|Vector|MakeVector 0.0 0.0 (Math|Float|SnapToGrid(Float) (* (Class|FastNoiseWrapper|GetNoise2D (Variables|/Game/Minecraft/BluePrints/GameModeTerrain.GameModeTerrain_C|GetNoise (Variables|Default|GetAs%20Game%20Mode%20Terrain)) (.x (+ (* (Variables|Default|GetChunkCoords) 16.0) (Math|Vector|MakeVector (Math|Conversions|ToFloat(Integer) _index) (Math|Conversions|ToFloat(Integer) _index_2) 0.0))) (.y (+ (* (Variables|Default|GetChunkCoords) 16.0) (Math|Vector|MakeVector (Math|Conversions|ToFloat(Integer) _index) (Math|Conversions|ToFloat(Integer) _index_2) 0.0)))) 1e+03) 1e+02))) "0, 0, 0" "1.000000,1.000000,1.000000") false))))))

(fn ConstructionScript)

(fn MakeStaticMesh
  (params (Input :type DA%20Base%20Object%20Reference))
  (bind _instancemap (Variables|Default|GetinstanceMap))
  (bind (_value _returnvalue) (Utilities|Map|Find _instancemap Input))
  (if _returnvalue
    (return _value)
    (else
      (bind _returnvalue_2 (AddComponent|AddInstanceStaticMeshBlock :DataAsset Input))
      (Utilities|Map|Add (Variables|Default|GetinstanceMap) Input _returnvalue_2)
      (return _returnvalue_2))))